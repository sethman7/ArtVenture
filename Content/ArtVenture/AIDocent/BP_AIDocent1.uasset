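; AI docent character for the ArtVenture VR experience that guides and advises the player on request.
; On BeginPlay it binds to VRPawn dispatchers for chase and advice, with UnTriggerDocentChase ending advice.
; The handlers only toggle guide and advice blackboard flags on its AI controller, leaving behavior to the AI logic that reads them.
; An older gaze-driven move-to-player and data-table text sequence remains unconnected.
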(event `self.ReceiveBeginPlay`
  (bind _returnvalue (`GameplayStatics.GetActorOfClass` "/Game/VRTemplate/Blueprints/VRPawn.VRPawn_C"))
  (add `/Game/VRTemplate/Blueprints/VRPawn.TriggerChase` _returnvalue (delegate `TriggerChase_Event`))
  (add `/Game/VRTemplate/Blueprints/VRPawn.UnTriggerChase` _returnvalue (delegate `UnTriggerChase`))
  (add `/Game/VRTemplate/Blueprints/VRPawn.TriggerDocentAdvice` _returnvalue (delegate `TriggerAdvice`))
  (add `/Game/VRTemplate/Blueprints/VRPawn.UnTriggerDocentChase` _returnvalue (delegate `UntriggerAdvice`)))

(event `TriggerChase_Event`
  (`BlackboardComponent.SetValueAsBool` (`AIBlueprintHelperLibrary.GetBlackboard` (`AIBlueprintHelperLibrary.GetAIController` self)) "DoesPlayerNeedGuide" true)
  (`BlackboardComponent.SetValueAsBool` (`AIBlueprintHelperLibrary.GetBlackboard` (`AIBlueprintHelperLibrary.GetAIController` self)) "HasGuidedPlayer" false))

(event `UnTriggerChase`
  (`BlackboardComponent.SetValueAsBool` (`AIBlueprintHelperLibrary.GetBlackboard` (`AIBlueprintHelperLibrary.GetAIController` self)) "DoesPlayerNeedGuide" false))

(event `TriggerAdvice`
  (`BlackboardComponent.SetValueAsBool` (`AIBlueprintHelperLibrary.GetBlackboard` (`AIBlueprintHelperLibrary.GetAIController` self)) "DoesPlayerNeedAdvice" true)
  (`BlackboardComponent.SetValueAsBool` (`AIBlueprintHelperLibrary.GetBlackboard` (`AIBlueprintHelperLibrary.GetAIController` self)) "HasAdvicedPlayer" false))

(event `UntriggerAdvice`
  (`BlackboardComponent.SetValueAsBool` (`AIBlueprintHelperLibrary.GetBlackboard` (`AIBlueprintHelperLibrary.GetAIController` self)) "DoesPlayerNeedAdvice" false))

(event `self.ReceiveTick`
  (params (DeltaSeconds :type "Float (single-precision)")))

(fn `UserConstructionScript`)