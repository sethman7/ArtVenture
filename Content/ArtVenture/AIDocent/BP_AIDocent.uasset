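; AI docent actor for ArtVenture that sends questions to an AI chat service and prints the replies on screen.
; BeginPlay creates a hidden WBP_AIDocentUI widget, and custom events show it with cursor and UI-only input, or hide it.
; Sphere overlap sets IsPlayer without filtering the actor, and leaving also hides the UI.
; Hiding does not restore game input mode.
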(event `self.ReceiveBeginPlay`
  (bind _returnvalue (`|CreateWidget` "/Game/ArtVenture/AIDocent/WBP_AIDocentUI.WBP_AIDocentUI_C" (`GameplayStatics.GetPlayerController` 0)))
  (`UserWidget.AddToViewport` _returnvalue 0)
  (`Widget.SetVisibility` _returnvalue "Hidden"))

(event `AskAIDocent`
  (params (Ask :type String :default "hello"))
  (bind (_asynctaskproxy _response) (`HttpGPTChatRequest.SendMessage_DefaultOptions` Ask)
    (:`ProcessCompleted`
      (if (`.bSuccess` (break `HttpGPTChatResponse` _response))
        (for _array_element (`.Choices` (break `HttpGPTChatResponse` _response))
          (`KismetSystemLibrary.PrintText` (`|FormatText` "{a}" (`.Content` (break `HttpGPTChatMessage` (`.Message` (break `HttpGPTChatChoice` _array_element))))) true true (struct :`G` 1.0 :`B` 0.026647 :`A` 1.0) 20.0))))))

(event `self.Sphere1.OnComponentBeginOverlap`
  (params (OverlappedComponent :type "PrimitiveComponent Object Reference") (OtherActor :type "Actor Object Reference") (OtherComp :type "PrimitiveComponent Object Reference") (OtherBodyIndex :type Integer) (bFromSweep :type Boolean) (SweepResult :type "HitResult Structure (by ref)"))
  (set `self.bIsPlayer` true))

(event `self.Sphere1.OnComponentEndOverlap`
  (params (OverlappedComponent :type "PrimitiveComponent Object Reference") (OtherActor :type "Actor Object Reference") (OtherComp :type "PrimitiveComponent Object Reference") (OtherBodyIndex :type Integer))
  (set `self.bIsPlayer` false)
  (`self.UI Invisibility`))

(event `UI Visibility`
  (bind _returnvalue (`GameplayStatics.GetPlayerController` 0))
  (`Widget.SetVisibility` (stale `self.ReceiveBeginPlay` _returnvalue) "Visible")
  (set `PlayerController.bShowMouseCursor` true _returnvalue)
  (`WidgetBlueprintLibrary.SetInputMode_UIOnlyEx` _returnvalue (stale `self.ReceiveBeginPlay` _returnvalue) "DoNotLock" true))

(event `UI Invisibility`
  (`Widget.SetVisibility` (stale `self.ReceiveBeginPlay` _returnvalue) "Hidden")
  (set `PlayerController.bShowMouseCursor` false (`GameplayStatics.GetPlayerController` 0)))

(fn `UserConstructionScript`)