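; BP_AIDocent is an AI docent actor that tries to follow the player and owns a hidden docent chat-style UI widget.
; Tick issues AIMoveTo at the player controller, and BeginPlay creates WBP_AIDocentUI.
; A sphere overlap sets IsPlayer without filtering the actor; leaving it also hides the UI.
; UIVisibility, not called here, shows the widget with cursor and UI-only input; UIInvisibility never restores input mode, and AskAIDocent is empty.
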(event `self.ReceiveTick`
  (params (DeltaSeconds :type "Float (single-precision)"))
  (`|ExecutionSequence`
    (:`then_0`
      (`|AIMoveTo` null (0.0 0.0 0.0) (`GameplayStatics.GetPlayerController` 0)))
    (:`then_1`
      (`KismetSystemLibrary.RetriggerableDelay` 1.0))))

(event `self.ReceiveBeginPlay`
  (bind _returnvalue (`|CreateWidget` "/Game/ArtVenture/AIDocent/Dummy/WBP_AIDocentUI.WBP_AIDocentUI_C" (`GameplayStatics.GetPlayerController` 0)))
  (`UserWidget.AddToViewport` _returnvalue 0)
  (`Widget.SetVisibility` _returnvalue "Hidden"))

(event `AskAIDocent`
  (params (Ask :type String :default "hello")))

(event `self.Sphere1.OnComponentBeginOverlap`
  (params (OverlappedComponent :type "PrimitiveComponent Object Reference") (OtherActor :type "Actor Object Reference") (OtherComp :type "PrimitiveComponent Object Reference") (OtherBodyIndex :type Integer) (bFromSweep :type Boolean) (SweepResult :type "HitResult Structure (by ref)"))
  (set `self.bIsPlayer` true))

(event `self.Sphere1.OnComponentEndOverlap`
  (params (OverlappedComponent :type "PrimitiveComponent Object Reference") (OtherActor :type "Actor Object Reference") (OtherComp :type "PrimitiveComponent Object Reference") (OtherBodyIndex :type Integer))
  (set `self.bIsPlayer` false)
  (`self.UI Invisibility`))

(event `UI Visibility`
  (bind _returnvalue (`GameplayStatics.GetPlayerController` 0))
  (`Widget.SetVisibility` (stale `self.ReceiveBeginPlay` _returnvalue) "Visible")
  (set `PlayerController.bShowMouseCursor` true _returnvalue)
  (`WidgetBlueprintLibrary.SetInputMode_UIOnlyEx` _returnvalue (stale `self.ReceiveBeginPlay` _returnvalue) "DoNotLock" true))

(event `UI Invisibility`
  (`Widget.SetVisibility` (stale `self.ReceiveBeginPlay` _returnvalue) "Hidden")
  (set `PlayerController.bShowMouseCursor` false (`GameplayStatics.GetPlayerController` 0)))

(fn `UserConstructionScript`)