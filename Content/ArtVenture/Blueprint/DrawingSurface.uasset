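; DrawingSurface is a Blueprint with a cube mesh that serves as a render-target canvas for brush drawing.
; Its construction script creates the render target, assigns it to a dynamic material on the cube, and creates a brush material instance from Mat_DrawingBrush.
; DrawBrush draws that brush onto the target, but Location is unwired and Size feeds screen position; the texture parameter name is also None.
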(fn `DrawBrush`
  (params (Size :type "Float (double-precision)") (Location :type "Vector2D Structure"))
  (bind _size (`local.Size`))
  (bind (_canvas _size_2 _context) (`KismetRenderingLibrary.BeginDrawCanvasToRenderTarget` (`self.RenderTarget`)))
  (`Canvas.K2_DrawMaterial` _canvas (`self.Brush`) (`KismetMathLibrary.MakeVector2D` _size _size) (0.0 0.0) (0.0 0.0) (1.0 1.0) 0.0 (0.5 0.5))
  (`KismetRenderingLibrary.EndDrawCanvasToRenderTarget` _context))

(fn `UserConstructionScript`
  (`|ExecutionSequence`
    (:`then_0`
      (bind _returnvalue (`KismetRenderingLibrary.CreateRenderTarget2D` 256))
      (set `self.RenderTarget` _returnvalue))
    (:`then_1`
      (bind _returnvalue_2 (`KismetMaterialLibrary.CreateDynamicMaterialInstance` (`PrimitiveComponent.GetMaterial` (`self.Cube`) 0)))
      (`MaterialInstanceDynamic.SetTextureParameterValue` _returnvalue_2 "None" (`self.RenderTarget`))
      (`PrimitiveComponent.SetMaterial` (`self.Cube`) 0 _returnvalue_2))
    (:`then_2`
      (bind _returnvalue_3 (`KismetMaterialLibrary.CreateDynamicMaterialInstance` "/Game/ArtVenture/Materials/Mat_DrawingBrush.Mat_DrawingBrush"))
      (set `self.Brush` _returnvalue_3))))